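; BP_EmailManager is an actor that periodically delivers random emails to the in-game monitor.
; A looping timer picks a random row from the DTEmail data table and spawns a BP_Email at the manager's transform.
; Each email receives the row data and a running index, then adds itself to the monitor.
; The manager also increments the email count on the player controller's MonitorUI.
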(event `self.ReceiveBeginPlay`
  (`KismetSystemLibrary.K2_SetTimer` null "Spawn Random Email" 4.0 true)
  (bind _asbp_player_controller (cast `/Game/Blueprints/BP_PlayerController` (`GameplayStatics.GetPlayerController` 0)))
  (set `self.BP Player Controller` _asbp_player_controller))

(event `Spawn Random Email`
  (bind _datatable (break `DataTableRowHandle` (`.EmailData_3_926B71CB4612F0E411C6B68D9E045967` (break `/Game/Email/S_Emails` (`self.DT Email`)))))
  (bind _outrownames (`DataTableFunctionLibrary.GetDataTableRowNames` _datatable))
  (bind _returnvalue (`|GetDataTableRow` _datatable (`|GetArrayItem` _outrownames (`KismetMathLibrary.RandomIntegerInRange` 0 (- (`KismetArrayLibrary.Array_Length` _outrownames) 1))))
    (:`then`
      (bind _returnvalue_2 (`|SpawnActorFromClass` "/Game/Email/BP_Email.BP_Email_C" (`self.GetTransform`) "Undefined" "MultiplyWithRoot" null null))
      (set `/Game/Email/BP_Email.Email Data` _returnvalue _returnvalue_2)
      (set `/Game/Email/BP_Email.Email Index` (`self.Email Index`) _returnvalue_2)
      (`/Game/Email/BP_Email.Add Email To Monitor` _returnvalue_2)
      (`/Engine/EditorBlueprintResources/StandardMacros.IncrementInt` (`self.Email Index`)
        (:`  `
          (`/Engine/EditorBlueprintResources/StandardMacros.IncrementInt` (`/Game/UI/Event/WBP_EventMonitorUI.Email Count` (`/Game/Blueprints/BP_PlayerController.MonitorUI` (`self.BP Player Controller`)))))))))

(fn `UserConstructionScript`)