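; BP_CyberEvent is an actor for a timed cyber event shown on the player's monitor UI.
; AddEventToMonitor sets the countdown from the event data's time limit, caches the player controller and registers the event with its MonitorUI.
; Tick decrements the remaining time and, on expiry, a DoOnce reports a timeout with name, type, damage and index to MonitorUI, then destroys the actor.
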(event `self.ReceiveBeginPlay`)

(event `AddEventToMonitor`
  (set `self.RemainingTime` (`.TimeLimit_12_35F2184D4DFD9BBE6CD42E9E95A6D207` (break `/Game/Event/S_CyberEventStruct` (`self.EventData`))))
  (bind _asbp_player_controller (cast `/Game/Blueprints/BP_PlayerController` (`GameplayStatics.GetPlayerController` 0)))
  (set `self.BP Player Controller` _asbp_player_controller)
  (`/Game/UI/Event/WBP_EventMonitorUI.AddEvent` (`/Game/Blueprints/BP_PlayerController.MonitorUI` _asbp_player_controller) self null))

(event `self.ReceiveTick`
  (params (DeltaSeconds :type "Float (single-precision)"))
  (bind (_eventname _eventtype _threatlevel _timelimit _canbesolved _solutionhint _damage) (break `/Game/Event/S_CyberEventStruct` (`self.EventData`)))
  (set `self.RemainingTime` (- (`self.RemainingTime`) DeltaSeconds))
  (if (<= (`self.RemainingTime`) 0.0)
    (`/Engine/EditorBlueprintResources/StandardMacros.DoOnce` false
      (:`Completed`
        (`/Game/UI/Event/WBP_EventMonitorUI.Timeout` (`/Game/Blueprints/BP_PlayerController.MonitorUI` (`self.BP Player Controller`)) _eventname _eventtype _damage (`self.EventIndex`))
        (`self.K2_DestroyActor`)))))

(fn `UserConstructionScript`)