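; BP_EventManager periodically spawns random cyber events and pushes them to the player's monitor UI.
; On BeginPlay it caches the BP_PlayerController and starts a looping timer at SpawnInterval.
; Each tick, if the monitor can accept an event, it picks a random data table row, spawns a BP_CyberEvent with that data and an incrementing index, tracks it in ActiveEvents, and adds it to the monitor.
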(event `self.ReceiveBeginPlay`
  (bind _asbp_player_controller (cast `/Game/Blueprints/BP_PlayerController` (`GameplayStatics.GetPlayerController` 0)))
  (set `self.BP Player Controller` _asbp_player_controller)
  (`KismetSystemLibrary.K2_SetTimer` null "SpawnRandomEvent" (`self.SpawnInterval`) true))

(event `SpawnRandomEvent`
  (bind _datatable (break `DataTableRowHandle` (`.EventData_4_3089351D419A46C5C9E693AB8F7778F4` (break `/Game/Event/S_Events` (`self.CyberEventDataTable`)))))
  (if (`/Game/UI/Event/WBP_EventMonitorUI.canAddEvent` (`/Game/Blueprints/BP_PlayerController.MonitorUI` (`self.BP Player Controller`)))
    (bind _outrownames (`DataTableFunctionLibrary.GetDataTableRowNames` _datatable))
    (bind _returnvalue (`|GetDataTableRow` _datatable (`|GetArrayItem` _outrownames (`KismetMathLibrary.RandomIntegerInRange` 0 (- (`KismetArrayLibrary.Array_Length` _outrownames) 1))))
      (:`then`
        (bind _returnvalue_2 (`|SpawnActorFromClass` "/Game/Event/BP_CyberEvent.BP_CyberEvent_C" (`self.GetTransform`) "Undefined" "MultiplyWithRoot" null null))
        (set `/Game/Event/BP_CyberEvent.EventData` _returnvalue _returnvalue_2)
        (`KismetArrayLibrary.Array_Add` (`self.ActiveEvents`) _returnvalue_2)
        (set `/Game/Event/BP_CyberEvent.EventIndex` (`self.EventIndex`) _returnvalue_2)
        (`/Game/Event/BP_CyberEvent.AddEventToMonitor` _returnvalue_2)
        (`/Engine/EditorBlueprintResources/StandardMacros.IncrementInt` (`self.EventIndex`))))))

(fn `UserConstructionScript`)