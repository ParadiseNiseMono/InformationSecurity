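; Manager actor that spawns the incident events belonging to the player's current stage.
; On BeginPlay it caches BP_PlayerController and runs a spawn pass over incident data table row names, looking each up in DT_IncidentEvent.
; Rows whose Stage matches the controller's PlayingStage each spawn a BP_IncidentEvent that receives the row data.
; Tick polls the controller's ChangeStageToAddingEvent flag to repeat the pass, then clears it.
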(event `self.ReceiveBeginPlay`
  (bind _asbp_player_controller (cast `/Game/Blueprints/BP_PlayerController` (`GameplayStatics.GetPlayerController` 0)))
  (set `self.As BP Player Controller` _asbp_player_controller)
  (`self.SpawnIncidentEvent`))

(event `self.ReceiveTick`
  (params (DeltaSeconds :type "Float (single-precision)"))
  (bind _as_bp_player_controller (`self.As BP Player Controller`))
  (if (`/Game/Blueprints/BP_PlayerController.Change Stage To Adding Event? ` _as_bp_player_controller)
    (`self.SpawnIncidentEvent`)
    (set `/Game/Blueprints/BP_PlayerController.Change Stage To Adding Event? ` false _as_bp_player_controller)))

(event `SpawnIncidentEvent`
  (bind _outrownames (`DataTableFunctionLibrary.GetDataTableRowNames` (`.DataTable` (break `DataTableRowHandle` (`.S_IncidentEvent_3_340BDAEB4E27E06BD8C138B471B3966E` (break `/Game/Event/IncidentEvent/S_IncidentEvents` (`self.S_IncidentEvents`)))))))
  (for _array_element _outrownames
    (bind _returnvalue (`|GetDataTableRow` "/Game/Event/IncidentEvent/DT_IncidentEvent.DT_IncidentEvent" _array_element)
      (:`then`
        (if (== (`.Stage_35_2AA8042B400694F9E39923AE1FCC256F` (break `/Game/Event/IncidentEvent/S_IncidentEvent` _returnvalue)) (`/Game/Blueprints/BP_PlayerController.PlayingStage` (`self.As BP Player Controller`)))
          (bind _returnvalue_2 (`|SpawnActorFromClass` "/Game/Event/IncidentEvent/BP_IncidentEvent.BP_IncidentEvent_C" (`self.Spawn Transform`) "Undefined" "MultiplyWithRoot" null null))
          (set `self.BP_IncidentEvent` _returnvalue_2)
          (set `/Game/Event/IncidentEvent/BP_IncidentEvent.IncidentEvent` _returnvalue (`self.BP_IncidentEvent`)))))))

(fn `UserConstructionScript`)