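; BP_IncidentEvent is an incident actor that plants a dangerous IP on a random staff member until the player blocks it.
; On BeginPlay it registers itself and its hint with the player's MonitorUI, then adds the IP to a staff's connections.
; AttackingStaff comes from a separate random roll and is never read.
; Tick polls the controller's BlockedIP; on a match it notifies MonitorUI and destroys itself.
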(event `self.ReceiveBeginPlay`
  (bind _asbp_player_controller (cast `/Game/Blueprints/BP_PlayerController` (`GameplayStatics.GetPlayerController` 0)))
  (set `self.As BP Player Controller` _asbp_player_controller)
  (`/Game/UI/Event/WBP_EventMonitorUI.AddEvent` (`/Game/Blueprints/BP_PlayerController.MonitorUI` (`self.As BP Player Controller`)) null self (`.Hint_15_D59C303F49A826A96C2EB6974700BDE4` (break `/Game/Event/trashs/IncidentEvent/S_IncidentEvent` (`self.IncidentEvent`))))
  (`self.AddDangerIpToRandomStaff`))

(event `AddDangerIpToRandomStaff`
  (bind _staffs (`/Game/UI/Staff/WBP_Staff.Staffs` (`/Game/Blueprints/BP_PlayerController.StaffUI` (`self.As BP Player Controller`))))
  (bind _output (`|GetArrayItem` _staffs (`KismetMathLibrary.RandomIntegerInRange` 0 (- (`KismetArrayLibrary.Array_Length` _staffs) 1))))
  (`KismetArrayLibrary.Array_Add` (`/Game/UI/Staff/WBP_StaffSlot.ConnectingIps` _output) (`.DangerIP_32_92B4AFEF49F71A1A66CD4FA486FD108D` (break `/Game/Event/trashs/IncidentEvent/S_IncidentEvent` (`self.IncidentEvent`))))
  (set `self.AttackingStaff` _output))

(event `self.ReceiveTick`
  (params (DeltaSeconds :type "Float (single-precision)"))
  (if (== (`/Game/Blueprints/BP_PlayerController.BlockedIP` (`self.As BP Player Controller`)) (`.IP_4_9710A82D4D8FC7CA2766E081CC26F076` (break `/Game/IPConnection/S_IPConnection` (`.DangerIP_32_92B4AFEF49F71A1A66CD4FA486FD108D` (break `/Game/Event/trashs/IncidentEvent/S_IncidentEvent` (`self.IncidentEvent`))))))
    (`/Game/UI/Event/WBP_EventMonitorUI.EventBeenHandled` (`/Game/Blueprints/BP_PlayerController.MonitorUI` (`self.As BP Player Controller`)) self)
    (`self.K2_DestroyActor`)))

(fn `UserConstructionScript`)