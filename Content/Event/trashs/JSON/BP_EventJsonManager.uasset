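; BP_EventJsonManager is an actor that periodically spawns random cyber events from JSON event data and sends them to the player's monitor UI.
; On BeginPlay it caches the BP_PlayerController and starts a looping SpawnInterval timer.
; Each tick of that timer, if MonitorUI allows another event, it picks a random data table row, spawns a BP_CyberEventJson with it, calls AddEventToMonitor and increments EventIndex.
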(event `self.ReceiveBeginPlay`
  (bind _asbp_player_controller (cast `/Game/Blueprints/BP_PlayerController` (`GameplayStatics.GetPlayerController` 0)))
  (set `self.BP Player Controller` _asbp_player_controller)
  (`KismetSystemLibrary.K2_SetTimer` null "SpawnRandomEvent" (`self.SpawnInterval`) true))

(event `SpawnRandomEvent`
  (bind _datatable (break `DataTableRowHandle` (`.EventJsonData_3_29E58B4B45198B6634A874B1B5E69267` (break `/Game/Event/trashs/JSON/S_CyberEventJsons` (`self.CyberEventJsonDataTable`)))))
  (if (`/Game/UI/Event/WBP_EventMonitorUI.canAddEvent` (`/Game/Blueprints/BP_PlayerController.MonitorUI` (`self.BP Player Controller`)))
    (bind _outrownames (`DataTableFunctionLibrary.GetDataTableRowNames` _datatable))
    (bind _returnvalue (`|GetDataTableRow` _datatable (`|GetArrayItem` _outrownames (`KismetMathLibrary.RandomIntegerInRange` 0 (- (`KismetArrayLibrary.Array_Length` _outrownames) 1))))
      (:`then`
        (bind _returnvalue_2 (`|SpawnActorFromClass` "/Game/Event/trashs/JSON/BP_CyberEventJson.BP_CyberEventJson_C" (`self.GetTransform`) "Undefined" "MultiplyWithRoot" null null))
        (set `/Game/Event/trashs/JSON/BP_CyberEventJson.EventDataJson` _returnvalue _returnvalue_2)
        (`/Game/Event/trashs/JSON/BP_CyberEventJson.AddEventToMonitor` _returnvalue_2)
        (`/Engine/EditorBlueprintResources/StandardMacros.IncrementInt` (`self.EventIndex`))))))

(fn `UserConstructionScript`)