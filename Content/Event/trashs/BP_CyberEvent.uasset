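; BP_CyberEvent is an actor for a timed cyber event, apparently meant to appear on the player controller's MonitorUI.
; AddEventToMonitor copies the time limit from EventData into RemainingTime and caches the BP_PlayerController.
; The countdown, which would report a timeout with damage and destroy the actor, is disconnected, as is the call adding the event to MonitorUI.
; BeginPlay and Tick are empty.
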(event `self.ReceiveBeginPlay`)

(event `AddEventToMonitor`
  (set `self.RemainingTime` (`.TimeLimit_12_35F2184D4DFD9BBE6CD42E9E95A6D207` (break `/Game/Event/trashs/S_CyberEventStruct` (`self.EventData`))))
  (bind _asbp_player_controller (cast `/Game/Blueprints/BP_PlayerController` (`GameplayStatics.GetPlayerController` 0)))
  (set `self.BP Player Controller` _asbp_player_controller))

(event `self.ReceiveTick`
  (params (DeltaSeconds :type "Float (single-precision)")))

(fn `UserConstructionScript`)