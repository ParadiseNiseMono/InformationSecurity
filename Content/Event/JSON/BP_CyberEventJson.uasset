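; BP_CyberEventJson is a timed cyber event built around randomly chosen JSON code snippets.
; On BeginPlay it spawns a random number of BP_JsonCode actors, fills each from a random data table row and collects those codes in an array.
; AddEventToMonitor registers the event with the player controller's monitor UI.
; Tick counts down RemainingTime, but expiry only reaches a DoOnce with no visible follow-up.
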(event `self.ReceiveBeginPlay`
  (`self.SpawnJsonCode`))

(event `AddEventToMonitor`
  (bind _asbp_player_controller (cast `/Game/Blueprints/BP_PlayerController` (`GameplayStatics.GetPlayerController` 0)))
  (set `self.BP Player Controller` _asbp_player_controller)
  (`/Game/UI/Event/WBP_EventMonitorUI.AddEvent` (`/Game/Blueprints/BP_PlayerController.MonitorUI` _asbp_player_controller) null self))

(event `self.ReceiveTick`
  (params (DeltaSeconds :type "Float (single-precision)"))
  (set `self.RemainingTime` (- (`self.RemainingTime`) DeltaSeconds))
  (if (<= (`self.RemainingTime`) 0.0)
    (`/Engine/EditorBlueprintResources/StandardMacros.DoOnce` false)))

(event `SpawnJsonCode`
  (bind _datatable (break `DataTableRowHandle` (`.JsonCode_2_FA34DB1B408426AFF2152E952B580B82` (break `/Game/Event/JSON/Json_Codes/S_JsonCodes` (`self.JsonCodes`)))))
  (for _ (range (+ (`KismetMathLibrary.RandomInteger` 100) 1))
    (bind _returnvalue (`|SpawnActorFromClass` "/Game/Event/JSON/Json_Codes/BP_JsonCode.BP_JsonCode_C" (`self.jsonCode Spawn Transform`) "Undefined" "MultiplyWithRoot" null null))
    (bind _outrownames (`DataTableFunctionLibrary.GetDataTableRowNames` _datatable))
    (bind _returnvalue_2 (`|GetDataTableRow` _datatable (`|GetArrayItem` _outrownames (`.OutIndex` (`KismetArrayLibrary.Array_Random` _outrownames))))
      (:`then`
        (bind _output_get (set `/Game/Event/JSON/Json_Codes/BP_JsonCode.JsonCode` _returnvalue_2 _returnvalue))
        (`KismetArrayLibrary.Array_Add` (`self.JsonCodeArray`) _output_get)))))

(fn `UserConstructionScript`)